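; Monster spawner component that tries to spawn a random AI monster around its owner on a looping one-second timer.
; Each tick picks a point on a circle scaled by Radius times pi and requires a short downward trace to hit world static or dynamic geometry.
; A random DT_Monstar row supplies the class, which spawns with BT_Mon and receives its stats through BP_MonsterBase's SetMonStat.
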(event `self.ReceiveBeginPlay`
  (`KismetSystemLibrary.K2_SetTimer` null "DoSpawn" 1.0 true))

(fn `DoSpawn`
  (locals (RandLocation :type "Vector Structure" :default (0.0 0.0 0.0)) (RandomLowName :type Name))
  (bind _output_get (set `local.RandLocation` (`self.GetRandomCircleRocation`)))
  (if (`self.IsCanSpawnLocation` _output_get)
    (bind _outrownames (`DataTableFunctionLibrary.GetDataTableRowNames` "/Game/HackandSlash/Monster/DT_Monstar.DT_Monstar"))
    (bind _output_get_2 (set `local.RandomLowName` (`KismetArrayLibrary.Array_Random` _outrownames)))
    (bind _returnvalue (`|GetDataTableRow` "/Game/HackandSlash/Monster/DT_Monstar.DT_Monstar" _output_get_2)
      (:`then`
        (bind _returnvalue_2 (`AIBlueprintHelperLibrary.SpawnAIFromClass` (`.MonsterClass_7_5CEA63E6412046FBE877DC972875A85F` (break `/Game/HackandSlash/Monster/ST_Monster` _returnvalue)) "/Game/HackandSlash/Monster/BT_Mon.BT_Mon" (`local.RandLocation`) (struct) false null))
        (bind _asbp_monster_base (cast `/Game/HackandSlash/Monster/BP_MonsterBase` _returnvalue_2))
        (`/Game/HackandSlash/Monster/BP_MonsterBase.SetMonStat` _asbp_monster_base _output_get_2)))))

(fn `GetRandomCircleRocation`
  (returns (ReturnValue :type "Vector Structure"))
  (locals (Rand :type "Float (double-precision)" :default 0.0))
  (bind _returnvalue (* (`self.Radius`) 3.141592))
  (bind _output_get (set `local.Rand` (`KismetMathLibrary.RandomFloatInRange` 0.0 360.0)))
  (return (+ (`Actor.K2_GetActorLocation` (`self.GetOwner`)) (`KismetMathLibrary.MakeVector` (* (`KismetMathLibrary.Cos` _output_get) _returnvalue) (* (`KismetMathLibrary.Sin` _output_get) _returnvalue)))))

(fn `IsCanSpawnLocation`
  (params (WorldLocation :type "Vector Structure"))
  (returns (IsCanSpawn :type Boolean))
  (bind (_outhit _returnvalue) (`KismetSystemLibrary.LineTraceSingleForObjects` WorldLocation (+ WorldLocation (0.0 0.0 -100.0)) (`|MakeArray` "ObjectTypeQuery1" "ObjectTypeQuery2" :!type "EObjectTypeQuery Enum")))
  (return _returnvalue))