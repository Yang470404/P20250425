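; BP_SkillMgr is a skill manager that automatically fires its owner's skills on repeating cooldowns.
; AddSkill copies a DT_Skill row into the Skills array with its timer already at the cooldown, so it triggers almost immediately.
; Tick advances each timer; once it exceeds the cooldown, DoUseSkill spawns the skill's class at the owner's transform, if the owner is a Character, and the timer resets.
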(event `self.ReceiveTick`
  (params (DeltaSeconds :type "Float (single-precision)"))
  (`self.UpdateSkills` DeltaSeconds))

(fn `AddSkill`
  (params (SkillRowName :type Name))
  (bind _returnvalue (`|GetDataTableRow` "/Game/HackandSlash/Skills/DT_Skill.DT_Skill" SkillRowName)
    (:`then`
      (bind (_name _skillclass _cooltime) (break `/Game/HackandSlash/Skills/ST_Skill` _returnvalue))
      (`KismetArrayLibrary.Array_Add` (`self.Skills`) (make `/Game/HackandSlash/Skills/ST_CurSkill` _returnvalue _cooltime))
      (`KismetSystemLibrary.PrintString` (`KismetStringLibrary.Concat_StrStr` "Add Skill - " _name) true true (struct :`R` 1.0 :`G` 0.071455 :`B` 0.739724 :`A` 1.0)))))

(fn `DoUseSkill`
  (params (CurSkill :type "/Game/HackandSlash/Skills/ST_CurSkill Structure"))
  (bind _returnvalue (`self.GetOwner`))
  ; log
  (`KismetSystemLibrary.PrintString` (`KismetStringLibrary.Concat_StrStr` "Use Skill - " (break `/Game/HackandSlash/Skills/ST_Skill` (`.SkillData_4_EB2417AC49AEA4DF4F67BB96743917A9` (break `/Game/HackandSlash/Skills/ST_CurSkill` CurSkill)))) true true (struct :`G` 0.66 :`B` 1.0 :`A` 1.0) 5.0)
  (cast `Character` _returnvalue)
  (`|SpawnActorFromClass` (`.SkillClass_7_0E700B4F436480AA95D03A9A57CB6765` (break `/Game/HackandSlash/Skills/ST_Skill` (`.SkillData_4_EB2417AC49AEA4DF4F67BB96743917A9` (break `/Game/HackandSlash/Skills/ST_CurSkill` CurSkill)))) (`Actor.GetTransform` _returnvalue) "Undefined" "MultiplyWithRoot" null null) ; SkillBase로 부모설정 + char변수 설정 했는데 Char가 안뜨네잉~~
)

(fn `UpdateSkillCoolTime`
  (params (InputPin :type "/Game/HackandSlash/Skills/ST_CurSkill Structure (by ref)") (DeltaSec :type "Float (double-precision)"))
  (bind _structout (setmembers `/Game/HackandSlash/Skills/ST_CurSkill` :`StructRef` InputPin :`CurCoolTime` (+ (`.CurCoolTime_6_9B4AD94F4AB2903CBB39A99815A96E41` (break `/Game/HackandSlash/Skills/ST_CurSkill` InputPin)) DeltaSec)))
  (bind (_skilldata _curcooltime) (break `/Game/HackandSlash/Skills/ST_CurSkill` _structout))
  (if (> _curcooltime (`.Cooltime_8_AF78C1FE48503FA764F5349181A659BC` (break `/Game/HackandSlash/Skills/ST_Skill` _skilldata)))
    (`self.DoUseSkill` _structout)
    (setmembers `/Game/HackandSlash/Skills/ST_CurSkill` :`StructRef` _structout :`CurCoolTime` 0.0)))

(fn `UpdateSkills`
  (params (DeltaSec :type "Float (double-precision)"))
  (for (_ _array_index) (`self.Skills`)
    (`self.UpdateSkillCoolTime` (`|GetArrayItem` (`self.Skills`) _array_index) DeltaSec)))