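; BP_Slash is a hack-and-slash skill actor that plays a slash effect on a character and deals damage.
; On BeginPlay it snaps a component to the character's mesh and applies radial damage at its own location, ignoring that character and crediting its controller.
; It binds to the Niagara system's finished event, with EventFinishAttack as the handler that destroys the actor.
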(event `self.ReceiveBeginPlay`
  (add `NiagaraComponent.OnSystemFinished` (`self.Niagara`) (`|CreateDelegate` :!event `EventFinishAttack`))
  (`self.K2_AttachToComponent` (`Character.Mesh` (`self.Char`)) "None" "SnapToTarget" "SnapToTarget" "SnapToTarget")
  (`GameplayStatics.ApplyRadialDamage` 10.0 (`self.K2_GetActorLocation`) 0.0 null (`|MakeArray` (`self.Char`) :!type "Actor Object Reference") self (`Pawn.GetController` (`self.Char`))))

(fn `EventFinishAttack`
  (params (PSystem :type "NiagaraComponent Object Reference"))
  (`self.K2_DestroyActor`))

(fn `UserConstructionScript`)